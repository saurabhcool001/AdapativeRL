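; BP_FloorDoor is a landing door for an elevator, with a call button and an outside floor display.
; CallElevator sends its FloorNumber to the linked BPElevator, animates the button press and tints the up and/or down text based on the car's current floor.
; The display updates through the elevator's FloorNumberSet event, bound at BeginPlay.
; OpenDoor and CloseDoor slide two panels in opposite directions by playing or reversing one timeline.
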(event Custom|CallElevator
  (bind _button (Variables|Default|GetButton))
  (bind _relativelocation (Variables|/Script/Engine.SceneComponent|GetRelativeLocation _button))
  ;[0 0 0] Call Elevator to the Floor
  (Utilities|IsValid (Variables|Default|GetBP_Elevator)
    (:Is%20Valid
      (Utilities|FlowControl|Sequence
        (:then_0
          (Default|FloorSelected (Variables|Default|GetBP_Elevator) (Variables|Default|GetFloorNumber)))
        (:then_1
          (Utilities|FlowControl|Sequence
            (:then_0
              (bind _position (Timeline|ButtonAnimationTimeline PlayFromStart)
                (:Update
                  (Transformation|SetRelativeLocation _button (Math|Vector|MakeVector (.x _relativelocation) (+ _position 9.0) (.z _relativelocation)) false false))))
            (:then_1
              (if (< (Variables|/Game/RealElevator/Blueprints/BP_Elevator.BP_Elevator_C|GetCurrentFloor (Variables|Default|GetBP_Elevator)) (Variables|Default|GetFloorNumber))
                (Rendering|Components|TextRender|SetTextRenderColor (Variables|Default|GetButtonTextUp) (Math|Color|MakeColor 255 100 0 255))
                (elif (> (Variables|/Game/RealElevator/Blueprints/BP_Elevator.BP_Elevator_C|GetCurrentFloor (Variables|Default|GetBP_Elevator)) (Variables|Default|GetFloorNumber))
                  (Rendering|Components|TextRender|SetTextRenderColor (Variables|Default|GetButtonTextDown) (Math|Color|MakeColor 255 100 0 255))
                  (else
                    (Rendering|Components|TextRender|SetTextRenderColor (Variables|Default|GetButtonTextDown) (Math|Color|MakeColor 255 100 0 255))))))))))))

(event Custom|OpenDoor
  ;[0 0 0] Open/Close Doors
  (bind _position (Timeline|DoorAnimationTimeline Play)
    (:Update
      (Utilities|FlowControl|Sequence
        (:then_0
          (Transformation|SetRelativeLocation (Variables|Default|GetDoorRight) (Math|Vector|MakeVector _position 0.0 6.532018) false false))
        (:then_1
          (Transformation|SetRelativeLocation (Variables|Default|GetDoorLeft) (Math|Vector|MakeVector (* _position -1.0) 0.0 6.532018) false false))))))

(event Custom|CloseDoor
  ;[0 0 0] Open/Close Doors
  (bind _position (Timeline|DoorAnimationTimeline Reverse)
    (:Update
      (Utilities|FlowControl|Sequence
        (:then_0
          (Transformation|SetRelativeLocation (Variables|Default|GetDoorRight) (Math|Vector|MakeVector _position 0.0 6.532018) false false))
        (:then_1
          (Transformation|SetRelativeLocation (Variables|Default|GetDoorLeft) (Math|Vector|MakeVector (* _position -1.0) 0.0 6.532018) false false))))))

(event Custom|CustomEvent
  (params (Floor :type Integer))
  ;[0 0 0] Get floor number from Elevator to display outside
  (Rendering|Components|TextRender|SetText (Variables|Default|GetFloorNumberDisplay) (Utilities|Text|ToText(Integer) Floor)))

(event EventBeginPlay
  ;[0 0 0] Get floor number from Elevator to display outside
  (EventDispatchers|BindEventtoFloorNumberSet (Variables|Default|GetBP_Elevator) (delegate Custom|CustomEvent)))

(fn ConstructionScript)
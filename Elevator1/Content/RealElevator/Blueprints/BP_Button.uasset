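; Elevator button panel that offers floor, open door, close door and stop buttons.
; ConfigureButtons spawns a grid of button meshes with number labels, tagging each with its floor number.
; ButtonClick uses that tag to color and animate the button, but calls FloorSelected over a fixed index range, as does ElevateLift, rather than passing the tagged floor.
; Door and stop events fire their own dispatchers, with timeline-driven presses and temporary label tints.
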(event Custom|StopElevator
  (bind _button3 (Variables|Default|GetButton3))
  (bind _relativelocation (Variables|/Script/Engine.SceneComponent|GetRelativeLocation _button3))
  ;[0 0 0] Stop Button
  (Rendering|Components|TextRender|SetTextRenderColor (Variables|Default|GetNumberDisplay3) (Math|Color|MakeColor 0 0 255 255))
  (Utilities|FlowControl|Sequence
    (:then_0
      (Default|CallStopButtonPressed))
    (:then_1
      (bind _position (Timeline|Timeline_2 PlayFromStart)
        (:Update
          (Transformation|SetRelativeLocation _button3 (Math|Vector|MakeVector (.x _relativelocation) (.y _relativelocation) _position) false false))
        (:Finished
          (Rendering|Components|TextRender|SetTextRenderColor (Variables|Default|GetNumberDisplay3) (Math|Color|MakeColor 255 255 255 255)))))))

(event Custom|ElevateLift
  (params (OverlappedComponent :type Primitive%20Component%20Object%20Reference) (OtherActor :type Actor%20Object%20Reference) (OtherComp :type Primitive%20Component%20Object%20Reference) (OtherBodyIndex :type Integer) (bFromSweep :type Boolean) (SweepResult :type Hit%20Result%20Structure%20%28by%20ref%29))
  (Utilities|FlowControl|Sequence
    (:then_0
      (for _index (range 1 10)
        (Default|CallFloorSelected _index)))))

(event Custom|OpenDoors
  (bind _button1 (Variables|Default|GetButton1))
  (bind _relativelocation (Variables|/Script/Engine.SceneComponent|GetRelativeLocation _button1))
  ;[0 0 0] Open Button
  (Rendering|Components|TextRender|SetTextRenderColor (Variables|Default|GetNumberDisplay1) (Math|Color|MakeColor 255 100 0 255))
  (Utilities|FlowControl|Sequence
    (:then_0
      (Default|CallOpenDoorsPressed))
    (:then_1
      (bind _position (Timeline|Timeline_0 PlayFromStart)
        (:Update
          (Transformation|SetRelativeLocation _button1 (Math|Vector|MakeVector (.x _relativelocation) (.y _relativelocation) _position) false false))
        (:Finished
          (Rendering|Components|TextRender|SetTextRenderColor (Variables|Default|GetNumberDisplay1) (Math|Color|MakeColor 255 255 255 255)))))))

(event Custom|ButtonClick
  (params (OverlappedComponent :type Primitive%20Component%20Object%20Reference) (OtherActor :type Actor%20Object%20Reference) (OtherComp :type Primitive%20Component%20Object%20Reference) (OtherBodyIndex :type Integer) (bFromSweep :type Boolean) (SweepResult :type Hit%20Result%20Structure%20%28by%20ref%29))
  (bind _buttonmeshes (Variables|Default|GetButtonMeshes))
  (bind _lowestfloor (Variables|Default|GetLowestFloor))
  (bind _componenttags (Variables|/Script/Engine.ActorComponent|GetComponentTags OverlappedComponent))
  (bind _output (Utilities|Array|Get(acopy) _componenttags))
  (bind _returnvalue (Utilities|String|ToString(Name) _output))
  (bind _returnvalue_2 (Math|Conversions|ToInteger(Byte) _returnvalue))
  (bind _returnvalue_3 (- _returnvalue_2 _lowestfloor))
  (bind _output_2 (Utilities|Array|Get(acopy) _buttonmeshes _returnvalue_3))
  (bind _relativelocation (Variables|/Script/Engine.SceneComponent|GetRelativeLocation _output_2))
  ;[0 0 0] ButtonPress
  (if (not (Components|ComponentHasTag OverlappedComponent "ignore"))
    (Utilities|FlowControl|Sequence
      (:then_0
        (Rendering|Components|TextRender|SetTextRenderColor (Utilities|Array|Get(acopy) (Variables|Default|GetTexts) _returnvalue_3) (Variables|Default|GetColor))
        (for _index (range 1 9)
          (Default|CallFloorSelected _index)))
      (:then_1
        (bind _position (Timeline|Timeline PlayFromStart)
          (:Update
            (Transformation|SetRelativeLocation _output_2 (Math|Vector|MakeVector (.x _relativelocation) (.y _relativelocation) _position) false false)))))))

(event Custom|CloseDoors
  (bind _button2 (Variables|Default|GetButton2))
  (bind _relativelocation (Variables|/Script/Engine.SceneComponent|GetRelativeLocation _button2))
  ;[0 0 0] Close Button
  (Rendering|Components|TextRender|SetTextRenderColor (Variables|Default|GetNumberDisplay2) (Math|Color|MakeColor 255 100 0 255))
  (Utilities|FlowControl|Sequence
    (:then_0
      (Default|CallCloseDoorsPressed))
    (:then_1
      (bind _position (Timeline|Timeline_1 PlayFromStart)
        (:Update
          (Transformation|SetRelativeLocation _button2 (Math|Vector|MakeVector (.x _relativelocation) (.y _relativelocation) _position) false false))
        (:Finished
          (Rendering|Components|TextRender|SetTextRenderColor (Variables|Default|GetNumberDisplay2) (Math|Color|MakeColor 255 255 255 255)))))))

(fn ConstructionScript)

(fn ConfigureButtons
  (params (NumberOfFloors :type Integer) (LowestFloor :type Integer) (ButtonsPerColumn :type Integer) (SpacingX :type Float%20%28double-precision%29) (SpacingY :type Float%20%28double-precision%29))
  (for _index (range 0 (- NumberOfFloors 1))
    (bind _returnvalue (AddComponent|AddStaticMeshComponent false))
    (Components|StaticMesh|SetStaticMesh _returnvalue "/Game/RealElevator/Meshes/SM_Elevator_Button.SM_Elevator_Button")
    (Variables|/Script/Engine.ActorComponent|SetComponentTags _returnvalue (Utilities|Array|MakeArray (Utilities|String|StringToName (Utilities|String|ToString(Integer) (+ _index LowestFloor)))))
    (Utilities|Array|Add (Variables|Default|GetButtonMeshes) _returnvalue)
    (Transformation|SetRelativeLocationAndRotation _returnvalue (Math|Vector|MakeVector (* (/ _index ButtonsPerColumn) SpacingX) (* (Math|Integer|%(Integer) _index ButtonsPerColumn) SpacingY) 0.0) "0, 0, 0" false false)
    (bind _returnvalue_2 (AddComponent|AddTextRenderComponent false))
    (Rendering|Components|TextRender|SetHorizontalAlignment _returnvalue_2 "EHTA_Center")
    (Class|TextRenderComponent|SetVerticalAlignment _returnvalue_2 "EVRTA_TextCenter")
    (Rendering|Components|TextRender|SetText _returnvalue_2 (Utilities|Text|ToText(Integer) (+ _index LowestFloor)))
    (Utilities|Array|Add (Variables|Default|GetTexts) _returnvalue_2)
    (Transformation|AttachComponentToComponent _returnvalue_2 _returnvalue "None" "KeepRelative" "KeepRelative" "KeepRelative" false)
    (Transformation|SetRelativeTransform _returnvalue_2 (Math|Transform|MakeTransform (Math|Vector|MakeVector (.x (Variables|/Script/Engine.SceneComponent|GetRelativeLocation _returnvalue_2)) (.y (Variables|/Script/Engine.SceneComponent|GetRelativeLocation _returnvalue_2)) 1.8) "90.000000,0.000000,0.000000" "0.150000,0.150000,0.150000") false false)))
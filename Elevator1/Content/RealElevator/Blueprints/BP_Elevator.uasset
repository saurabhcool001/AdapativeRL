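; Elevator car actor that carries the player between floors, driven by a child button panel it configures and binds for doors, floor selection and stop.
; Selected floors queue in press order; Tick moves the car at constant speed, then eases into the target height.
; That final easing waits until a "TriggerLift" UDP message has set LiftStatus.
; A timeline slides the car doors, while box overlaps find each BP_FloorDoor to operate and update floor displays.
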(event OnComponentBeginOverlap(Box)
  (params (OverlappedComponent :type Primitive%20Component%20Object%20Reference) (OtherActor :type Actor%20Object%20Reference) (OtherComp :type Primitive%20Component%20Object%20Reference) (OtherBodyIndex :type Integer) (bFromSweep :type Boolean) (SweepResult :type Hit%20Result%20Structure%20%28by%20ref%29))
  ;[0 0 0] Show Current Floor No. on all displays
  (if (Components|ComponentHasTag OtherComp "Door")
    (bind _asbp_floor_door (Utilities|Casting|CastToBP_FloorDoor OtherActor))
    (Rendering|Components|TextRender|SetText (Variables|Default|GetFloorNumberDisplay) (Utilities|Text|ToText(Integer) (Variables|/Game/RealElevator/Blueprints/BP_FloorDoor.BP_FloorDoor_C|GetFloorNumber _asbp_floor_door)))
    (Default|CallFloorNumberSet (Variables|/Game/RealElevator/Blueprints/BP_FloorDoor.BP_FloorDoor_C|GetFloorNumber _asbp_floor_door))))

(event OnMessageReceived(VRUDP)
  (params (Message :type String))
  ;[0.4806 0.2825 1] UDP Communication
  (if (Utilities|Enum|Equal(Enum) Message "TriggerLift")
    (Variables|Default|SetLiftStatus true)
    (Class|VRUDPComponent|SendUDPMessage (Variables|Default|GetVRUDP) "Lift moving")))

(event Custom|openDoor
  ;[0 0 0] Doors Open/Close Mechanism
  (if (not (Variables|Default|GetisMoving?))
    (CallFunction|OpenFloorDoor)
    (Utilities|FlowControl|Sequence
      (:then_0
        (Variables|Default|SetDoorClosing false)
        (bind _position (Timeline|OpenDoorAnimation Play)
          (:Update
            (Variables|Default|SetDoorsMoving true)
            (Utilities|FlowControl|Sequence
              (:then_0
                (Transformation|SetRelativeLocation (Variables|Default|GetDoor_Right) (Math|Vector|MakeVector (* _position -1.0) 2.3e+02 6.532018) false false))
              (:then_1
                (Transformation|SetRelativeLocation (Variables|Default|GetDoor_Left) (Math|Vector|MakeVector _position 2.3e+02 6.532018) false false))))
          (:Finished
            (if (Variables|Default|GetDoorClosing)
              (Variables|Default|SetDoorsMoving false)
              (Utilities|FlowControl|Delay (Variables|ElevatorSetting|GetOperationDelay))
              (CallFunction|MoveElevator)))))
      (:then_1
        (Utilities|FlowControl|Delay 7.0)
        (CallFunction|CloseDoor)))))

(event Custom|CloseDoor
  ;[0 0 0] Doors Open/Close Mechanism
  (Variables|Default|SetDoorClosing true)
  (CallFunction|CloseFloorDoor)
  (bind _position (Timeline|OpenDoorAnimation Reverse)
    (:Update
      (Variables|Default|SetDoorsMoving true)
      (Utilities|FlowControl|Sequence
        (:then_0
          (Transformation|SetRelativeLocation (Variables|Default|GetDoor_Right) (Math|Vector|MakeVector (* _position -1.0) 2.3e+02 6.532018) false false))
        (:then_1
          (Transformation|SetRelativeLocation (Variables|Default|GetDoor_Left) (Math|Vector|MakeVector _position 2.3e+02 6.532018) false false))))
    (:Finished
      (if (Variables|Default|GetDoorClosing)
        (Variables|Default|SetDoorsMoving false)
        (Utilities|FlowControl|Delay (Variables|ElevatorSetting|GetOperationDelay))
        (CallFunction|MoveElevator)))))

(event Custom|FloorSelected
  (params (Floors :type Integer))
  ;[0 0 0] Select and store selected Floor numbers
  (Utilities|Array|AddUnique (Variables|Default|GetSelectedFloors) Floors)
  (CallFunction|CloseDoor))

(event Custom|MoveElevator
  ;[0 0 0] Set variables before moving elevator
  (if (Utilities|Array|IsNotEmpty (Variables|Default|GetSelectedFloors))
    (Variables|Default|SetCurrentTargetHeight (+ (* (Utilities|Array|Get(acopy) (Variables|Default|GetSelectedFloors) (Variables|Default|GetTargetFloorIndex)) (Variables|ElevatorSetting|GetFloorHeight)) (- (Variables|Default|GetInitialHeight) (* (Variables|ElevatorSetting|GetFloorHeight) (Variables|ElevatorSetting|GetInitialFloor)))))
    (Variables|Default|SetisMoving? true)))

(event Custom|ArrivedAtFloor
  ;[0 0 0] Arrived At Selected Floor
  (Variables|ElevatorSetting|SetCurrentFloor (Utilities|Array|Get(acopy) (Variables|Default|GetSelectedFloors) (Variables|Default|GetTargetFloorIndex)))
  (CallFunction|OpenDoor)
  (Utilities|FlowControl|Sequence
    (:then_0
      (Utilities|FlowControl|Delay (+ (Variables|ElevatorSetting|GetOperationDelay) 2.0))
      (bind _output_get (Variables|Default|SetTargetFloorIndex (+ (Variables|Default|GetTargetFloorIndex) 1)))
      (if (Utilities|Array|IsValidIndex (Variables|Default|GetSelectedFloors) _output_get)
        (CallFunction|CloseDoor)
        (Variables|Default|SetLiftStatus false)
        (else
          (Variables|Default|SetisMoving? false)
          (Utilities|Array|Clear (Variables|Default|GetSelectedFloors))
          (Variables|Default|SetTargetFloorIndex 0)
          (CallFunction|CloseDoor))))))

(event Custom|Stop
  ;[0 0 0] Imergency Stop
  (if (Variables|Default|GetisMoving?)
    (Variables|Default|SetisMoving? false)
    (else
      (CallFunction|MoveElevator))))

(event EventBeginPlay
  (bind _bp_button (Variables|Default|Getbp_button))
  ;[0 0 0] Initialize
  (Utilities|IsValid _bp_button
    (:Is%20Valid
      (EventDispatchers|BindEventtoOpenDoorsPressed _bp_button (EventDispatchers|CreateEvent :!event Custom|openDoor))
      (EventDispatchers|BindEventtoCloseDoorsPressed _bp_button (EventDispatchers|CreateEvent :!event Custom|CloseDoor))
      (EventDispatchers|BindEventtoFloorSelected _bp_button (EventDispatchers|CreateEvent :!event Custom|FloorSelected))
      (EventDispatchers|BindEventtoStopButtonPressed _bp_button (EventDispatchers|CreateEvent :!event Custom|Stop))
      (Variables|Default|SetInitialHeight (.z (Transformation|GetActorLocation)))
      (Variables|ElevatorSetting|SetCurrentFloor (Variables|ElevatorSetting|GetInitialFloor))
      ;[0 0 0] Show Current Floor No. on all displays
      (bind _asbp_floor_door (Utilities|Casting|CastToBP_FloorDoor (Utilities|Array|Get(acopy) (Collision|GetOverlappingActors (Variables|Default|GetBox) "/Game/RealElevator/Blueprints/BP_FloorDoor.BP_FloorDoor_C" :!class /Script/Engine.PrimitiveComponent))))
      (Rendering|Components|TextRender|SetText (Variables|Default|GetFloorNumberDisplay) (Utilities|Text|ToText(Integer) (Variables|/Game/RealElevator/Blueprints/BP_FloorDoor.BP_FloorDoor_C|GetFloorNumber _asbp_floor_door)))
      (Default|CallFloorNumberSet (Variables|/Game/RealElevator/Blueprints/BP_FloorDoor.BP_FloorDoor_C|GetFloorNumber _asbp_floor_door)))))

(event EventTick
  (params (DeltaSeconds :type Float%20%28single-precision%29))
  (bind _returnvalue (Transformation|GetActorLocation))
  (bind _returnvalue_2 (Transformation|GetActorLocation))
  (bind _currenttargetheight (Variables|Default|GetCurrentTargetHeight))
  (bind _currenttargetheight_2 (Variables|Default|GetCurrentTargetHeight))
  ;[0 0 0] Start Moving Elevator
  (if (and (Variables|Default|GetisMoving?) (not (Variables|Default|GetDoorsMoving)))
    (if (Variables|Default|GetApplyBreak)
      (if (Variables|Default|GetLiftStatus)
        (Transformation|SetActorLocation (Math|Vector|MakeVector (.x _returnvalue) (.y _returnvalue) (Math|Interpolation|FInterpTo (.z _returnvalue) _currenttargetheight DeltaSeconds (Variables|ElevatorSetting|GetSpeed))) false false)
        (if (Math|Float|NearlyEqual(Float) (.z _returnvalue) _currenttargetheight 1.0)
          (Variables|Default|SetApplyBreak false)
          (Variables|Default|SetisMoving? false)
          (CallFunction|ArrivedatFloor)))
      (else
        (Transformation|SetActorLocation (Math|Vector|MakeVector (.x _returnvalue_2) (.y _returnvalue_2) (Math|Interpolation|FInterptoConstant (.z _returnvalue_2) _currenttargetheight_2 DeltaSeconds (* (Variables|ElevatorSetting|GetSpeed) 1.5e+02))) false false)
        (if (Math|Float|NearlyEqual(Float) (.z _returnvalue_2) _currenttargetheight_2 1e+02)
          (Variables|Default|SetApplyBreak true))))))

(fn ConstructionScript
  (bind _asbp_button (Utilities|Casting|CastToBP_Button (Variables|/Script/Engine.ChildActorComponent|GetChildActor (Variables|Default|GetBP_Button1))))
  (bind _output_get (Variables|Default|Setbp_button _asbp_button))
  (Variables|/Game/RealElevator/Blueprints/BP_Button.BP_Button_C|SetLowestFloor _output_get (Variables|ConfigureButton|GetLowest%20Floor))
  (Default|ConfigureButtons _output_get (Variables|ConfigureButton|GetNumber%20Of%20Floors) (Variables|ConfigureButton|GetLowest%20Floor) (Variables|ConfigureButton|GetButtons%20Per%20Column) (Variables|ConfigureButton|GetSpacing%20X) (Variables|ConfigureButton|GetSpacing%20Y)))

(fn SortArrayAscending
  (params (InputArray :type Array%20of%20Integers))
  (LocalVariables|SetLastIndex (Utilities|Array|Length InputArray))
  (bind _output_get (LocalVariables|SetLastIndex (- (stale _output_get) 1) :!label _label))
  (if (> _output_get 1)
    (for _index (range 1 (LocalVariables|GetLastIndex))
      (if (> (Utilities|Array|Get(acopy) InputArray (- _index 1)) (Utilities|Array|Get(acopy) InputArray _index))
        (Utilities|Array|Swap InputArray _index (- _index 1))))
    (goto _label)))

(fn OpenFloorDoor
  (bind _asbp_floor_door (Utilities|Casting|CastToBP_FloorDoor (Utilities|Array|Get(acopy) (Collision|GetOverlappingActors (Variables|Default|GetBox) "/Game/RealElevator/Blueprints/BP_FloorDoor.BP_FloorDoor_C" :!class /Script/Engine.PrimitiveComponent))))
  (Rendering|Components|TextRender|SetTextRenderColor (Variables|/Game/RealElevator/Blueprints/BP_FloorDoor.BP_FloorDoor_C|GetButtonTextUp _asbp_floor_door) (Math|Color|MakeColor 255 255 255 255))
  (Default|OpenDoor _asbp_floor_door))

(fn CloseFloorDoor
  (bind _asbp_floor_door (Utilities|Casting|CastToBP_FloorDoor (Utilities|Array|Get(acopy) (Collision|GetOverlappingActors (Variables|Default|GetBox) "/Game/RealElevator/Blueprints/BP_FloorDoor.BP_FloorDoor_C" :!class /Script/Engine.PrimitiveComponent))))
  (Default|CloseDoor _asbp_floor_door))